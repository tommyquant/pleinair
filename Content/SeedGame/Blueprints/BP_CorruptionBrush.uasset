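; Temporary brush actor that paints into the corruption map render targets at its location, offset by a global parameter collection vector.
; A looping timer feeds color, position, radius and density into a dynamic material, optionally growing the radius with each draw.
; Each draw renders the brush into RT_CorruptionMapB, then M_Transfer into RT_CorruptionMapA, and the actor destroys itself after MaxDraws.
; The construction script sizes the sphere component to the brush radius.
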(event `self.ReceiveBeginPlay`
  (bind _returnvalue (`KismetMaterialLibrary.CreateDynamicMaterialInstance` "/Game/SeedGame/ParticleSystems/Materials/M_CorruptionBrush.M_CorruptionBrush"))
  (set `self.BrushMaterial` _returnvalue)
  (bind _returnvalue_2 (`KismetSystemLibrary.K2_SetTimerDelegate` (delegate `DrawBrush`) (`self.DrawInterval`) true))
  (set `self.TimerHandle` _returnvalue_2))

(event `DrawBrush`
  (bind (_brushcolor_x _brushcolor_y _brushcolor_z _brushcolor_w) (`KismetMathLibrary.BreakVector4` (`self.BrushColor`)))
  (bind _brushmaterial (`self.BrushMaterial`))
  (bind _returnvalue (`KismetMaterialLibrary.GetVectorParameterValue` "/Game/SeedGame/Materials/MPC_Global.MPC_Global" "CorruptionMapOffset"))
  (`MaterialInstanceDynamic.SetVectorParameterValue` _brushmaterial "Color" (make `LinearColor` _brushcolor_x _brushcolor_y _brushcolor_z _brushcolor_w))
  (`MaterialInstanceDynamic.SetVectorParameterValue` _brushmaterial "Location" (`KismetMathLibrary.Conv_VectorToLinearColor` (- (`self.K2_GetActorLocation`) (`KismetMathLibrary.Conv_LinearColorToVector` _returnvalue))))
  (`MaterialInstanceDynamic.SetScalarParameterValue` _brushmaterial "Radius" (* (`self.BrushRadius`) (`KismetMathLibrary.SelectFloat` (/ (`KismetMathLibrary.Conv_IntToDouble` (+ (`self.DrawCount`) 1)) (`KismetMathLibrary.Conv_IntToDouble` (`self.MaxDraws`))) 1.0 (`self.StepSize`))))
  (`MaterialInstanceDynamic.SetScalarParameterValue` _brushmaterial "Density" (`self.BrushDensity`))
  (`KismetRenderingLibrary.DrawMaterialToRenderTarget` "/Game/SeedGame/Textures/RT_CorruptionMapB.RT_CorruptionMapB" (`self.BrushMaterial`))
  (`KismetRenderingLibrary.DrawMaterialToRenderTarget` "/Game/SeedGame/Textures/RT_CorruptionMapA.RT_CorruptionMapA" "/Game/SeedGame/ParticleSystems/Materials/M_Transfer.M_Transfer")
  (bind _result (`/Engine/EditorBlueprintResources/StandardMacros.IncrementInt` (`self.DrawCount`))
    (:`  `
      (if (>= _result (`self.MaxDraws`))
        (`KismetSystemLibrary.K2_ClearAndInvalidateTimerHandle` (`self.TimerHandle`))
        (`self.K2_DestroyActor`)))))

(fn `UserConstructionScript`
  (`SphereComponent.SetSphereRadius` (`self.Sphere`) (`self.BrushRadius`) false))