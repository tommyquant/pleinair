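; Corruption crystal actor that spreads corruption within a set radius until it is cured.
; On BeginPlay it registers with its Tree, spawns a corruption brush at its sphere using its radius and density, and creates a dynamic material for the mesh.
; Curing runs only while corrupted, calling CallCureCrystal and playing a timeline that drives the material's CrystalState.
; The construction script sizes the sphere to the corruption radius.
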(event `self.ReceiveBeginPlay`
  (`/Game/SeedGame/Blueprints/BP_Tree.AddCrystal` (`self.Tree`) self)
  (`|SpawnActorFromClass` "/Game/SeedGame/Blueprints/BP_CorruptionBrush.BP_CorruptionBrush_C" (`KismetMathLibrary.MakeTransform` (`SceneComponent.K2_GetComponentLocation` (`self.Sphere`))) "Undefined" "OverrideRootScale" self (1.0 0.0 0.0 0.0) (`self.CorruptionRadius`) (`self.CorruptionDensity`) 0.01 1 false null)
  (bind _returnvalue (`KismetMaterialLibrary.CreateDynamicMaterialInstance` "/Game/SeedGame/Materials/Crystals/MI_Crystal_01.MI_Crystal_01"))
  (bind _output_get (set `self.CrystalMaterial` _returnvalue))
  (`PrimitiveComponent.SetMaterial` (`self.CrystalMesh`) 0 _output_get))

(event `OnCured`
  (if (`self.IsCorrupted`)
    (set `self.IsCorrupted` false)
    (`self.CureCrystal`)
    (bind (_direction _alpha) (`Timeline|CureTimeline` :!via `PlayFromStart`)
      (:`Update`
        (`MaterialInstanceDynamic.SetScalarParameterValue` (`self.CrystalMaterial`) "CrystalState" _alpha)))))

(fn `UserConstructionScript`
  (`SphereComponent.SetSphereRadius` (`self.Sphere`) (`self.CorruptionRadius`) false))