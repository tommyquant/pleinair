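; Player actor: a constantly gliding paper plane that steers by look input, boosts speed and drops random flower seeds on a cooldown.
; Tick moves it with per-axis sweeps, while one boost alpha blends speed, camera zoom, MPC radial blur and audio.
; A downward landscape trace sets grass rustle volume.
; It spawns a particle capture showing only BrushParticles, publishes its location to MPC_Global, and FreeRoam destroys the level bounds.
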(event `self.ReceiveBeginPlay`
  (`AudioComponent.FadeIn` (`self.AmbientWind`) 2.0 1.0 0.0)
  (bind _returnvalue (`|SpawnActorFromClass` "/Game/SeedGame/Blueprints/BP_ParticleCapture.BP_ParticleCapture_C" (`KismetMathLibrary.MakeTransform` (0.0 0.0 0.0)) "AlwaysSpawn" "OverrideRootScale" self self null))
  (`SceneCaptureComponent.ShowOnlyComponent` (`/Game/SeedGame/Blueprints/BP_ParticleCapture.SceneCaptureComponent2D` _returnvalue) (`self.BrushParticles`)))

(event `self.ReceiveTick`
  (params (DeltaSeconds :type "Float (single-precision)"))
  (`|ExecutionSequence`
    (:`then_0`
      (`self.CalculateSpeedMultiplier`)
      (`self.ZoomCamera`)
      (`self.BlurCamera`)
      (`self.ProcessMovement`)
      (`self.UpdateTrailParticles`)
      (`self.UpdateAudio`))
    (:`then_1`
      (`KismetMaterialLibrary.SetVectorParameterValue` "/Game/SeedGame/Materials/MPC_Global.MPC_Global" "PlaneLocation" (`KismetMathLibrary.Conv_VectorToLinearColor` (`self.K2_GetActorLocation`))))))

(event `InputAxis|SpeedUp`
  (params (AxisValue :type "Float (single-precision)"))
  (if (> AxisValue 0.0)
    (set `self.IsSpeedingUp` true)
    (else
      (set `self.IsSpeedingUp` false))))

(event `InputAxis|DropSeed`
  (params (AxisValue :type "Float (single-precision)"))
  (if (and (`self.CanDropSeed`) (> AxisValue 0.0))
    (`|SpawnActorFromClass` "/Game/SeedGame/Blueprints/BP_DropSeed.BP_DropSeed_C" (`KismetMathLibrary.MakeTransform` (`SceneComponent.K2_GetComponentLocation` (`self.DropSeedLocation`))) "Undefined" "OverrideRootScale" self (`KismetMathLibrary.RandomIntegerInRange` 1 3) (`self.DropSeedRadius`) null)
    (set `self.CanDropSeed` false)
    (`KismetSystemLibrary.Delay` (`self.DropInterval`))
    (set `self.CanDropSeed` true)))

(event `InputAxis|TurnHorizontal`
  (params (AxisValue :type "Float (single-precision)"))
  (bind _returnvalue (* AxisValue (`self.MouseSensitivity`)))
  (`|ExecutionSequence`
    (:`then_0`
      (`self.AddControllerYawInput` _returnvalue))
    (:`then_1`
      (`self.SetPlaneRoll` _returnvalue))
    (:`then_2`
      (`self.SetCameraOffset` _returnvalue))))

(event `InputAxis|TurnVertical`
  (params (AxisValue :type "Float (single-precision)"))
  (`self.AddControllerPitchInput` (* AxisValue (`self.MouseSensitivity`))))

(event `InputAction|FreeRoam`
  (params (Key :type "Key Structure"))
  (:`Pressed`
    (bind _outactors (`GameplayStatics.GetAllActorsOfClass` "/Game/SeedGame/Blueprints/BP_Bounds.BP_Bounds_C"))
    (bind _output (`|GetArrayItem` _outactors))
    (`/Engine/EditorBlueprintResources/StandardMacros.IsValid` _output
      (:`Is Valid`
        (`self.K2_DestroyActor` _output)
        (`KismetSystemLibrary.PrintString` "Free roam activated — enjoy your stay!" true true (struct :`G` 0.66 :`B` 1.0 :`A` 1.0) 10.0)))))

(fn `BlurCamera`
  (`KismetMaterialLibrary.SetScalarParameterValue` "/Game/SeedGame/Materials/MPC_PostProcess.MPC_PostProcess" "RadialBlurAlpha" (`self.SpeedTransitionAlpha`)))

(fn `CalculateSpeedMultiplier`
  (set `self.SpeedTransitionAlpha` (`KismetMathLibrary.FClamp` (+ (`self.SpeedTransitionAlpha`) (* (`GameplayStatics.GetWorldDeltaSeconds`) (`KismetMathLibrary.SelectFloat` (`self.SpeedTransitionStartScale`) (`self.SpeedTransitionStopScale`) (`self.IsSpeedingUp`)))))))

(fn `ProcessMovement`
  (locals (MoveOffset :type "Vector Structure"))
  (bind (_moveoffset_x _moveoffset_y _moveoffset_z) (`KismetMathLibrary.BreakVector` (`local.MoveOffset`)))
  (bind _speed (`self.Speed`))
  (bind _moveoffset_x_2 (`KismetMathLibrary.BreakVector` (`local.MoveOffset`)))
  (bind (_moveoffset_x_3 _moveoffset_y_2) (`KismetMathLibrary.BreakVector` (`local.MoveOffset`)))
  (bind (_returnvalue_x _returnvalue_y _returnvalue_z) (`KismetMathLibrary.BreakVector` (* (`self.GetActorForwardVector`) (`KismetMathLibrary.Lerp` _speed (* _speed (`self.SpeedMultiplier`)) (`self.SpeedTransitionAlpha`)))))
  (set `self.LastLocation` (`self.K2_GetActorLocation`))
  (set `local.MoveOffset` (* (+ (`KismetMathLibrary.MakeVector` _returnvalue_x _returnvalue_y _returnvalue_z) (`self.AdditionalOffset`)) (`GameplayStatics.GetWorldDeltaSeconds`)))
  (`self.K2_AddActorWorldOffset` (`KismetMathLibrary.MakeVector` _moveoffset_x_2) true)
  (`self.K2_AddActorWorldOffset` (`KismetMathLibrary.MakeVector` 0.0 _moveoffset_y_2) true)
  (`self.K2_AddActorWorldOffset` (`KismetMathLibrary.MakeVector` 0.0 0.0 _moveoffset_z) true))

(fn `SetCameraOffset`
  (params (AxisValue :type "Float (double-precision)"))
  (bind _cameramaxoffset (`self.CameraMaxOffset`))
  (bind (_relativelocation_x _relativelocation_y) (`KismetMathLibrary.BreakVector` (`SceneComponent.RelativeLocation` (`self.Camera`))))
  (`SceneComponent.K2_SetRelativeLocation` (`self.Camera`) (`KismetMathLibrary.MakeVector` 0.0 (`KismetMathLibrary.FClamp` (+ AxisValue _relativelocation_y) (* _cameramaxoffset -1.0) _cameramaxoffset)) false false))

(fn `SetPlaneRoll`
  (params (AxisValue :type "Float (double-precision)"))
  (bind (_relativerotation_roll _relativerotation_pitch) (`KismetMathLibrary.BreakRotator` (`SceneComponent.RelativeRotation` (`self.PaperPlaneMesh`))))
  (set `self.TargetRoll` (* AxisValue (`self.MaxRoll`) -1.0))
  (`SceneComponent.K2_SetRelativeRotation` (`self.PaperPlaneMesh`) (`KismetMathLibrary.MakeRotator` 0.0 (`KismetMathLibrary.FInterpTo` _relativerotation_pitch (`self.TargetRoll`) (`GameplayStatics.GetWorldDeltaSeconds`) (`self.RollInterpSpeed`)) 90.0) false false))

(fn `UpdateAudio`
  (bind _returnvalue (`self.K2_GetActorLocation`))
  (bind _grassrustle (`self.GrassRustle`))
  (`AudioComponent.SetFloatParameter` (`self.AmbientWind`) "Crossfade" (`self.SpeedTransitionAlpha`))
  (bind _outhit (`KismetSystemLibrary.LineTraceSingle` _returnvalue (- _returnvalue (`KismetMathLibrary.MakeVector` 0.0 0.0 (`self.GrassAudioDistance`))) "TraceTypeQuery1"))
  (bind (_bblockinghit _binitialoverlap _time _distance _location _impactpoint _normal _impactnormal _physmat _hitactor) (`GameplayStatics.BreakHitResult` _outhit))
  (cast `Landscape` _hitactor)
  (bind (_returnvalue_x _returnvalue_y _returnvalue_z) (`KismetMathLibrary.BreakVector` (- (`self.K2_GetActorLocation`) _location)))
  (`AudioComponent.SetVolumeMultiplier` _grassrustle (- 1.0 (`KismetMathLibrary.FClamp` (/ _returnvalue_z (`self.GrassAudioDistance`)))))
  (`AudioComponent.SetPitchMultiplier` _grassrustle (`KismetMathLibrary.Lerp` 1.0 10.0 (`self.SpeedTransitionAlpha`))))

(fn `UpdateTrailParticles`
  (bind _trail1 (`self.Trail1`))
  (if (`self.IsSpeedingUp`)
    (`ActorComponent.Activate` _trail1 false)
    (else
      (`ActorComponent.Deactivate` _trail1))))

(fn `UserConstructionScript`)

(fn `ZoomCamera`
  (set `SpringArmComponent.TargetArmLength` (`KismetMathLibrary.Lerp` (`self.CameraMinZoom`) (`self.CameraMaxZoom`) (`CurveFloat.GetFloatValue` (`self.CameraZoomCurve`) (`self.SpeedTransitionAlpha`))) (`self.SpringArm`)))