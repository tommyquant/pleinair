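; BP_Tree is a tree that can start corrupted and is cured once all crystals registered with it are cured.
; On BeginPlay it creates bark and leaf dynamic materials, registers with BP_PersistentActor and, if corrupted, spawns a BP_CorruptionBrush sized by CorruptionRadius.
; Crystal cure events increment a count; completion spawns an inverse brush, plays effects, fires TreeCured and runs a timeline driving both materials' TreeState.
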(event `self.ReceiveBeginPlay`
  (bind _treemesh (`self.TreeMesh`))
  (`|ExecutionSequence`
    (:`then_0`
      (bind _returnvalue (`KismetMaterialLibrary.CreateDynamicMaterialInstance` (`PrimitiveComponent.GetMaterial` (`self.TreeMesh`) 1)))
      (bind _output_get (set `self.TreeMaterial` _returnvalue))
      (`MaterialInstanceDynamic.SetScalarParameterValue` _output_get "TreeState" 0.0)
      (`PrimitiveComponent.SetMaterial` _treemesh 1 (`self.TreeMaterial`))
      (bind _returnvalue_2 (`KismetMaterialLibrary.CreateDynamicMaterialInstance` (`PrimitiveComponent.GetMaterial` _treemesh 0)))
      (bind _output_get_2 (set `self.LeafMaterial` _returnvalue_2))
      (`MaterialInstanceDynamic.SetScalarParameterValue` _output_get_2 "TreeState" 0.0)
      (`PrimitiveComponent.SetMaterial` (`self.TreeMesh`) 0 (`self.LeafMaterial`))
      (bind _outactors (`GameplayStatics.GetAllActorsOfClass` "/Game/SeedGame/Blueprints/BP_PersistentActor.BP_PersistentActor_C"))
      (`/Game/SeedGame/Blueprints/BP_PersistentActor.BindTreeDispatcher` (`|GetArrayItem` _outactors) self))
    (:`then_1`
      (if (`self.IsCorrupted`)
        (`|SpawnActorFromClass` "/Game/SeedGame/Blueprints/BP_CorruptionBrush.BP_CorruptionBrush_C" (`KismetMathLibrary.MakeTransform` (`self.K2_GetActorLocation`)) "Undefined" "OverrideRootScale" self (1.0 0.0 0.0 0.0) (`self.CorruptionRadius`) (`self.CorruptionDensity`) 0.01 1 false null)))))

(event `AddCrystal`
  (params (NewCrystal :type "/Game/SeedGame/Blueprints/BP_CorruptionCrystal Object Reference"))
  (`KismetArrayLibrary.Array_Add` (`self.Crystals`) NewCrystal)
  (`/Engine/EditorBlueprintResources/StandardMacros.IncrementInt` (`self.CrystalCount`)
    (:`  `
      (add `/Game/SeedGame/Blueprints/BP_CorruptionCrystal.CureCrystal` NewCrystal (delegate `OnCrystalCured`)))))

(event `OnCrystalCured`
  (bind _result (`/Engine/EditorBlueprintResources/StandardMacros.IncrementInt` (`self.CrystalsCured`))
    (:`  `
      (if (>= _result (`self.CrystalCount`))
        (`self.OnTreeCured`)))))

(event `OnTreeCured`
  (`|ExecutionSequence`
    (:`then_0`
      (set `self.IsCorrupted` false)
      (`|SpawnActorFromClass` "/Game/SeedGame/Blueprints/BP_CorruptionBrush.BP_CorruptionBrush_C" (`KismetMathLibrary.MakeTransform` (`self.K2_GetActorLocation`)) "Undefined" "OverrideRootScale" self (`KismetMathLibrary.MakeVector4` -1.0 0.0 (/ (`KismetMathLibrary.Conv_IntToDouble` (`KismetMathLibrary.RandomIntegerInRange` 1 3)) 255.0)) (`self.CorruptionRadius`) (`self.CorruptionDensity`) 0.05 5 true null)
      (`GameplayStatics.SpawnEmitterAtLocation` "/Game/SeedGame/ParticleSystems/PS_CureSphere.PS_CureSphere" (`self.K2_GetActorLocation`) (struct) (5.0 5.0 5.0))
      (`GameplayStatics.PlaySound2D` "/Game/SeedGame/Audio/S_Ding_01.SFX_Ding_001")
      (`self.TreeCured`))
    (:`then_1`
      (bind (_direction _tree _leaf) (`Timeline|TreeRevive` :!via `PlayFromStart`)
        (:`Update`
          (`MaterialInstanceDynamic.SetScalarParameterValue` (`self.TreeMaterial`) "TreeState" _tree)
          (`MaterialInstanceDynamic.SetScalarParameterValue` (`self.LeafMaterial`) "TreeState" _leaf))))))

(fn `UserConstructionScript`
  (`SphereComponent.SetSphereRadius` (`self.CorruptionSphere`) (`self.CorruptionRadius`) false))