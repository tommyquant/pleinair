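; Persistent game manager that runs the main menu, music and level flow for a tree-curing game.
; It swaps streamed levels around widget fades, possesses each level's player and reopens PersistentLevel after the last.
; Tree-cured events stop the timer, update per-level best times and unlock next-level input, alongside restart and quit.
; Each tick fades the corruption map by drawing materials through two render targets, cleared on level load.
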(event `self.ReceiveBeginPlay`
  (`|ExecutionSequence`
    (:`then_0`
      (`AudioComponent.FadeIn` (`self.Music`) 2.0 1.0 0.0)
      (for _array_element (`self.MinimumTimes`)
        (`KismetArrayLibrary.Array_Add` (`self.BestTimes`) _array_element)))
    (:`then_1`
      (bind _returnvalue (`|CreateWidget` "/Game/SeedGame/UI/WBP_MainMenu.WBP_MainMenu_C" null self))
      (bind _output_get (set `self.MainMenu` _returnvalue))
      (`UserWidget.AddToViewport` _output_get 0)
      (`self.SetMenuVisiblity` true))
    (:`then_2`
      (bind _returnvalue_2 (`KismetMaterialLibrary.CreateDynamicMaterialInstance` "/Game/SeedGame/ParticleSystems/Materials/M_FlowerTransitionFade.M_FlowerTransitionFade"))
      (set `self.FadeMaterial` _returnvalue_2))
    (:`then_3`
      (`self.OnStartLoad` (`self.CurrentLevel`)))))

(event `self.ReceiveTick`
  (params (DeltaSeconds :type "Float (single-precision)"))
  (bind _fadematerial (`self.FadeMaterial`))
  (`MaterialInstanceDynamic.SetScalarParameterValue` _fadematerial "FadeAmount" (* (`self.FadeAmount`) (`GameplayStatics.GetWorldDeltaSeconds`)))
  (`KismetRenderingLibrary.DrawMaterialToRenderTarget` "/Game/SeedGame/Textures/RT_CorruptionMapB.RT_CorruptionMapB" _fadematerial)
  (`KismetRenderingLibrary.DrawMaterialToRenderTarget` "/Game/SeedGame/Textures/RT_CorruptionMapA.RT_CorruptionMapA" "/Game/SeedGame/ParticleSystems/Materials/M_Transfer.M_Transfer")
  (if (< (`self.TreesCured`) (`self.MaxTrees`))
    (set `self.Timer` (+ (`self.Timer`) (`GameplayStatics.GetWorldDeltaSeconds`)))))

(event `OnStartLoad`
  (params (NextLevel :type Integer))
  (bind _output_get (set `self.NextLevel` NextLevel))
  (set `self.LoadingLevel` true)
  (if (> _output_get 0)
    (`/Game/SeedGame/UI/WBP_MainMenu.DoFade` (`self.MainMenu`) false)
    (else
      (`self.OnLoadNextLevel`))))

(event `OnLoadNextLevel`
  (`|ExecutionSequence`
    (:`then_0`
      (set `self.LoadingLevel` false)
      (if (> (`self.NextLevel`) 0)
        (`GameplayStatics.UnloadStreamLevel` (`|GetArrayItem` (`self.LevelList`) (`self.CurrentLevel`))))
      (bind _output_get (set `self.CurrentLevel` (`self.NextLevel`)))
      (bind _output (`|GetArrayItem` (`self.LevelList`) _output_get))
      (if (== _output "None")
        (`GameplayStatics.OpenLevel` "PersistentLevel")
        (else
          (`GameplayStatics.LoadStreamLevel` _output true true)
          (`KismetSystemLibrary.Delay` 0.1)
          (bind _outactors (`GameplayStatics.GetAllActorsOfClass` "/Game/SeedGame/Blueprints/BP_Player.BP_Player_C"))
          (bind _output_2 (`|GetArrayItem` _outactors))
          (`/Engine/EditorBlueprintResources/StandardMacros.IsValid` _output_2
            (:`Is Valid`
              (`Controller.Possess` (`GameplayStatics.GetPlayerController` 0) _output_2)
              (`self.SetMenuVisiblity` false)
              (`/Game/SeedGame/UI/WBP_MainMenu.DoFade` (`self.MainMenu`) true))
            (:`Is Not Valid`
              (`/Game/SeedGame/UI/WBP_MainMenu.DoFade` (`self.MainMenu`) true))))))
    (:`then_1`
      (`KismetRenderingLibrary.ClearRenderTarget2D` "/Game/SeedGame/Textures/RT_CorruptionMapA.RT_CorruptionMapA" (struct :`G` 1.0 :`A` 1.0))
      (`KismetRenderingLibrary.ClearRenderTarget2D` "/Game/SeedGame/Textures/RT_CorruptionMapB.RT_CorruptionMapB" (struct :`G` 1.0 :`A` 1.0))
      (`/Game/SeedGame/UI/WBP_MainMenu.SetNextLevelVisibility` (`self.MainMenu`) false))
    (:`then_2`
      (set `self.TreesCured` 0)
      (set `self.Timer` 0.0))))

(event `BindTreeDispatcher`
  (params (Tree :type "/Game/SeedGame/Blueprints/BP_Tree Object Reference"))
  (add `/Game/SeedGame/Blueprints/BP_Tree.TreeCured` Tree (delegate `OnTreeCured`))
  (set `self.MaxTrees` 1))

(event `OnTreeCured`
  (bind _result (`/Engine/EditorBlueprintResources/StandardMacros.IncrementInt` (`self.TreesCured`))
    (:`  `
      (if (>= _result (`self.MaxTrees`))
        (`|ExecutionSequence`
          (:`then_0`
            (if (< (`self.Timer`) (`|GetArrayItem` (`self.BestTimes`) (`self.CurrentLevel`)))
              (`KismetArrayLibrary.Array_Set` (`self.BestTimes`) (`self.CurrentLevel`) (`self.Timer`))))
          (:`then_1`
            (`/Game/SeedGame/UI/WBP_MainMenu.SetNextLevelVisibility` (`self.MainMenu`) true)))))))

(event `InputAction|NextLevel`
  (params (Key :type "Key Structure"))
  (:`Pressed`
    (if (>= (`self.TreesCured`) (`self.MaxTrees`))
      (`self.OnStartLoad` (+ (`self.CurrentLevel`) 1)))))

(event `InputAction|RestartLevel`
  (params (Key :type "Key Structure"))
  (:`Pressed`
    (if (> (`self.CurrentLevel`) 0)
      (`self.OnStartLoad` (`self.CurrentLevel`)))))

(event `InputAction|QuitGame`
  (params (Key :type "Key Structure"))
  (:`Pressed`
    (`KismetSystemLibrary.QuitGame` null "Quit")))

(fn `SetMenuVisiblity`
  (params (IsVisible :type Boolean))
  (bind _returnvalue (`GameplayStatics.GetPlayerController` 0))
  (bind _menupanel (`/Game/SeedGame/UI/WBP_MainMenu.MenuPanel` (`self.MainMenu`)))
  (bind _menupanel_2 (`/Game/SeedGame/UI/WBP_MainMenu.MenuPanel` (`self.MainMenu`)))
  (if IsVisible
    (`WidgetBlueprintLibrary.SetInputMode_UIOnlyEx` _returnvalue)
    (set `PlayerController.bShowMouseCursor` true _returnvalue)
    (`Widget.SetRenderOpacity` _menupanel 1.0)
    (`Widget.SetVisibility` _menupanel "SelfHitTestInvisible")
    (else
      (`WidgetBlueprintLibrary.SetInputMode_GameOnly` _returnvalue)
      (set `PlayerController.bShowMouseCursor` false _returnvalue)
      (`Widget.SetRenderOpacity` _menupanel_2 0.0)
      (`Widget.SetVisibility` _menupanel_2 "Hidden"))))

(fn `UserConstructionScript`)