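; BP_DropSeed is a falling seed actor that cures corruption crystals and spawns corruption brushes where it lands.
; Tick moves it down with a sweep; any overlap or sphere hit destroys it.
; Overlapping a corrupted crystal cures it with effects and spawns a brush using the crystal's radius and density.
; Non-crystal overlaps spawn a brush at the seed, with a random flower type encoded in brush color either way.
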(event `self.ReceiveActorBeginOverlap`
  (params (OtherActor :type "Actor Object Reference"))
  (set `self.FlowerType` (`KismetMathLibrary.RandomIntegerInRange` 1 3))
  (`|ExecutionSequence`
    (:`then_0`
      (bind _asbp_corruption_crystal (cast `/Game/SeedGame/Blueprints/BP_CorruptionCrystal` OtherActor)
        (:`then`
          (if (`/Game/SeedGame/Blueprints/BP_CorruptionCrystal.IsCorrupted` _asbp_corruption_crystal)
            (`/Game/SeedGame/Blueprints/BP_CorruptionCrystal.OnCured` _asbp_corruption_crystal)
            (set `self.Radius` (`/Game/SeedGame/Blueprints/BP_CorruptionCrystal.CorruptionRadius` _asbp_corruption_crystal))
            (set `self.Density` (`/Game/SeedGame/Blueprints/BP_CorruptionCrystal.CorruptionDensity` _asbp_corruption_crystal))
            (bind _returnvalue (`self.K2_GetActorLocation` _asbp_corruption_crystal))
            (`GameplayStatics.SpawnEmitterAtLocation` "/Game/SeedGame/ParticleSystems/PS_CureSphere.PS_CureSphere" _returnvalue)
            (`GameplayStatics.PlaySoundAtLocation` "/Game/SeedGame/Audio/S_CureSphere_Cue.S_CureSphere_Cue" _returnvalue)
            (`|SpawnActorFromClass` "/Game/SeedGame/Blueprints/BP_CorruptionBrush.BP_CorruptionBrush_C" (`KismetMathLibrary.MakeTransform` (`SceneComponent.K2_GetComponentLocation` (`/Game/SeedGame/Blueprints/BP_CorruptionCrystal.Sphere` _asbp_corruption_crystal))) "Undefined" "OverrideRootScale" self (`KismetMathLibrary.MakeVector4` -0.33 -1.0 (/ (`KismetMathLibrary.Conv_IntToDouble` (`self.FlowerType`)) 255.0)) (`self.Radius`) (`self.Density`) 0.05 3 false null)))
        (:`CastFailed`
          (`|SpawnActorFromClass` "/Game/SeedGame/Blueprints/BP_CorruptionBrush.BP_CorruptionBrush_C" (`KismetMathLibrary.MakeTransform` (`self.K2_GetActorLocation`)) "Undefined" "OverrideRootScale" self (`KismetMathLibrary.MakeVector4` -1.0 -1.0 (/ (`KismetMathLibrary.Conv_IntToDouble` (`self.FlowerType`)) 255.0)) (`self.Radius`) (`self.Density`) 0.01 1 false null))))
    (:`then_1`
      (`self.K2_DestroyActor`))))

(event `self.ReceiveTick`
  (params (DeltaSeconds :type "Float (single-precision)"))
  (`self.K2_AddActorWorldOffset` (`KismetMathLibrary.MakeVector` 0.0 0.0 (* DeltaSeconds (`self.FallSpeed`) -1.0)) true))

(event `self.Sphere.OnComponentHit`
  (params (HitComponent :type "PrimitiveComponent Object Reference") (OtherActor :type "Actor Object Reference") (OtherComp :type "PrimitiveComponent Object Reference") (NormalImpulse :type "Vector Structure") (Hit :type "HitResult Structure (by ref)"))
  (`self.K2_DestroyActor`))

(fn `UserConstructionScript`)